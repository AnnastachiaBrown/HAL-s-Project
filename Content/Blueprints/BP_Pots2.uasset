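; BP_Pots2 is an interactable plant pot that the first-person character seeds, then waters to grow a flower in stages.
; OnInteract checks the player's seed or watering can, plays Niagara on watering and consumes the can, but leaves HasSeed set.
; OnUpdate uses the watering count to reveal a fern, then swap bluebell meshes, re-enabling watering each stage.
; An overlap volume shows the prompt while unwatered, although IsInteractable always returns false.
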(event `self.InteractionCollision.OnComponentBeginOverlap`
  (params (OverlappedComponent :type "PrimitiveComponent Object Reference") (OtherActor :type "Actor Object Reference") (OtherComp :type "PrimitiveComponent Object Reference") (OtherBodyIndex :type Integer) (bFromSweep :type Boolean) (SweepResult :type "HitResult Structure (by ref)"))
  ; InteractionPrompt
  (cast `/Game/FirstPerson/Blueprints/BP_FirstPersonCharacter` OtherActor)
  (if (not (`self.wasWatered`))
    (`SceneComponent.SetVisibility` (`self.InteractionPrompt`) true false)))

(event `self.InteractionCollision.OnComponentEndOverlap`
  (params (OverlappedComponent :type "PrimitiveComponent Object Reference") (OtherActor :type "Actor Object Reference") (OtherComp :type "PrimitiveComponent Object Reference") (OtherBodyIndex :type Integer))
  ; InteractionPrompt
  (cast `/Game/FirstPerson/Blueprints/BP_FirstPersonCharacter` OtherActor)
  (`SceneComponent.SetVisibility` (`self.InteractionPrompt`) false false))

(event `self.OnInteract`
  (params (InteractingPlayer :type "Character Object Reference"))
  ; Watering/seedingthepot
  (bind _asbp_first_person_character (cast `/Game/FirstPerson/Blueprints/BP_FirstPersonCharacter` InteractingPlayer))
  (if (`self.WasSeeded`)
    (if (`/Game/FirstPerson/Blueprints/BP_FirstPersonCharacter.HasWaterCan` _asbp_first_person_character)
      (if (`self.wasWatered`)
        (`KismetSystemLibrary.PrintString` "You have Watered this plant already" true true (struct :`R` 0.495466 :`G` 0.143479 :`B` 0.143479 :`A` 1.0))
        (else
          (set `self.wasWatered` true)
          (set `self.waterTimes` (+ (`self.waterTimes`) 1))
          (`ActorComponent.Activate` (`self.Niagara`) false)
          (set `/Game/FirstPerson/Blueprints/BP_FirstPersonCharacter.HasWaterCan` false _asbp_first_person_character)
          (`KismetSystemLibrary.PrintString` "WateredPot" true true (struct :`R` 0.021003 :`G` 1.0 :`A` 1.0))))
      (else
        (`KismetSystemLibrary.PrintString` "YouDoNotHaveTheWateringCan")))
    (elif (`/Game/FirstPerson/Blueprints/BP_FirstPersonCharacter.HasSeed` _asbp_first_person_character)
      (set `self.WasSeeded` true)
      (`KismetSystemLibrary.PrintString` "Seed Planted" true true (struct :`R` 0.115875 :`G` 1.0 :`A` 1.0))
      (set `/Game/FirstPerson/Blueprints/BP_FirstPersonCharacter.HasSeed` true _asbp_first_person_character)
      (else
        (`KismetSystemLibrary.PrintString` "YouHaveNotPlantedASeedInThisPot" true true (struct :`R` 1.0 :`G` 0.139065 :`A` 1.0) 4.0)))))

(event `self.OnUpdate`
  (params (Player :type "/Game/FirstPerson/Blueprints/BP_FirstPersonCharacter Object Reference"))
  ; UpdatingFlower
  (switch `int` (`self.waterTimes`)
    (:`1`
      (`self.FlowerUpdate` null)
      (`SceneComponent.SetVisibility` (`self.fern`) true false))
    (:`2`
      (`self.FlowerUpdate` null)
      (`StaticMeshComponent.SetStaticMesh` (`self.FlowerMesh`) "/Game/VRS_LowPolyNature/Meshes/Env/Plants/Bluebells/SM_BluebellASimple.SM_BluebellASimple"))
    (:`3`
      (`self.FlowerUpdate` null)
      (`StaticMeshComponent.SetStaticMesh` (`self.FlowerMesh`) "/Game/VRS_LowPolyNature/Meshes/Env/Plants/Bluebells/SM_BluebellBLeaves.SM_BluebellBLeaves"))))

(event `FlowerUpdate`
  (params (Player :type "/Game/FirstPerson/Blueprints/BP_FirstPersonCharacter Object Reference"))
  ; UpdatingFlower
  (`KismetSystemLibrary.PrintString` (`KismetStringLibrary.Concat_StrStr` (`KismetStringLibrary.Conv_IntToString` (`self.waterTimes`)) ": FlowerUpdate"))
  (set `self.wasWatered` false))

(fn `IsInteractable`
  (returns (Interactable :type Boolean))
  (return false))

(fn `UserConstructionScript`)