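; BP_WaterCan is an interactable water can that the first-person character can pick up.
; Overlapping its InteractionCollision shows a widget for that character and hides it on exit.
; OnInteract sets a PickedUpWater flag and prints it, without removing or attaching the actor.
; IsInteractable always returns false, and draft logic for changing a widget image is left unconnected.
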(event `self.InteractionCollision .OnComponentBeginOverlap`
  (params (OverlappedComponent :type "PrimitiveComponent Object Reference") (OtherActor :type "Actor Object Reference") (OtherComp :type "PrimitiveComponent Object Reference") (OtherBodyIndex :type Integer) (bFromSweep :type Boolean) (SweepResult :type "HitResult Structure (by ref)"))
  (cast `/Game/FirstPerson/Blueprints/BP_FirstPersonCharacter` OtherActor)
  (`SceneComponent.SetVisibility` (`self.Widget`) true false))

(event `self.InteractionCollision .OnComponentEndOverlap`
  (params (OverlappedComponent :type "PrimitiveComponent Object Reference") (OtherActor :type "Actor Object Reference") (OtherComp :type "PrimitiveComponent Object Reference") (OtherBodyIndex :type Integer))
  (cast `/Game/FirstPerson/Blueprints/BP_FirstPersonCharacter` OtherActor)
  (`SceneComponent.SetVisibility` (`self.Widget`) false false))

(event `/Game/Blueprints/Interaction/BPI_Interact.OnInteract`
  (params (InteractingPlayer :type "Character Object Reference"))
  (bind _output_get (set `self.PickedUpWater` true))
  (`KismetSystemLibrary.PrintString` (`KismetStringLibrary.Conv_BoolToString` _output_get)))

(fn `IsInteractable`
  (returns (Interactable :type Boolean))
  (return false))

(fn `UserConstructionScript`)