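; Door actor that shows a prompt widget when the first-person character is near and opens a testing UI when interacted with.
; Sphere overlap events toggle the widget's visibility.
; OnInteract adds W_TestingPurposes to the player screen, switches to UI-only input with the cursor shown, and calls OnChangeMessage on the player controller.
; IsInteractable and OnChange are stubs returning false, and no door movement is implemented.
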(event `self.Sphere.OnComponentBeginOverlap`
  (params (OverlappedComponent :type "PrimitiveComponent Object Reference") (OtherActor :type "Actor Object Reference") (OtherComp :type "PrimitiveComponent Object Reference") (OtherBodyIndex :type Integer) (bFromSweep :type Boolean) (SweepResult :type "HitResult Structure (by ref)"))
  (cast `/Game/FirstPerson/Blueprints/BP_FirstPersonCharacter` OtherActor)
  (`SceneComponent.SetVisibility` (`self.Widget`) true false))

(event `self.Sphere.OnComponentEndOverlap`
  (params (OverlappedComponent :type "PrimitiveComponent Object Reference") (OtherActor :type "Actor Object Reference") (OtherComp :type "PrimitiveComponent Object Reference") (OtherBodyIndex :type Integer))
  (cast `/Game/FirstPerson/Blueprints/BP_FirstPersonCharacter` OtherActor)
  (`SceneComponent.SetVisibility` (`self.Widget`) false false))

(event `/Game/Blueprints/Interaction/BPI_Interact.OnInteract`
  (params (InteractingPlayer :type "Character Object Reference"))
  (bind _returnvalue (`GameplayStatics.GetPlayerController` 0))
  (bind _returnvalue_2 (`|CreateWidget` "/Game/Widgets/W_TestingPurposes.W_TestingPurposes_C"))
  (`UserWidget.AddToPlayerScreen` _returnvalue_2 0)
  (`WidgetBlueprintLibrary.SetInputMode_UIOnlyEx` _returnvalue null)
  (set `PlayerController.bShowMouseCursor` true _returnvalue)
  (message `/Game/Blueprints/Interaction/BPI_Update.OnChange` _returnvalue))

(fn `IsInteractable`
  (returns (Interactable :type Boolean))
  (return false))

(fn `OnChange`
  (returns (PlayerLeft :type Boolean))
  (return false))

(fn `UserConstructionScript`)